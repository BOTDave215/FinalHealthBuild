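; BP_Side2Side is an AI antibody wall actor that slides along its local Y axis and breaks down as it takes hits.
; Tick applies a fixed negative Y offset without sweep or delta-time scaling, so it never reverses and its speed follows frame rate.
; TakeHit drives a MultiGate that removes SkeletalMesh2, then SkeletalMesh1, then the actor, with a DoOnce and short Delay debouncing rapid hits.
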(event Custom|TakeHit
  (Utilities|FlowControl|Sequence
    (:then_0
      (Utilities|FlowControl|DoOnce false :!label _label
        (:Completed
          (Utilities|FlowControl|MultiGate false false -1
            (:Out%200
              (Components|DestroyComponent (Variables|Default|GetSkeletalMesh2)))
            (:Out%201
              (Components|DestroyComponent (Variables|Default|GetSkeletalMesh1)))
            (:Out%202
              (Actor|DestroyActor))))))
    (:then_1
      (Utilities|FlowControl|Delay 0.2)
      (goto _label Reset))))

(event EventBeginPlay)

(event Collision|EventActorBeginOverlap
  (params (OtherActor :type Actor%20Object%20Reference)))

(event EventTick
  (params (DeltaSeconds :type Float%20%28single-precision%29))
  (Transformation|AddActorLocalOffset "0,-5.000000, 0" false false))

(fn ConstructionScript)