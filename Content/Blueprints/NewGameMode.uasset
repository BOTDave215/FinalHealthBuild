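; Game mode that handles startup setup, tutorial help screens and switching between the tutorial level and Level1 by index.
; On BeginPlay it fills a pollution info array with numbered strings and forces graphics scalability to the lowest level.
; After a delay, if the player character is flagged as tutorial, it shows character, enemy and goal help widgets in turn.
; Each widget pauses the game, with a short Delay before its removal and no unpause here.
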(event Custom|OpenLevelLevel
  (params (currentLevel :type Integer))
  (switch int currentLevel
    (:0
      (Game|OpenLevel(byName) "TutLevel"))
    (:1
      (Game|OpenLevel(byName) "Level1"))))

(event EventBeginPlay
  (Utilities|FlowControl|Sequence
    (:then_0
      (Variables|Default|SetPollution%20Info (Utilities|Array|MakeArray "1" "2" "3" "4" "5" "6" "7")))
    (:then_1
      (bind _returnvalue (Settings|GetGameUserSettings))
      (Class|GameUserSettings|SetOverallScalabilityLevel _returnvalue)
      (Class|GameUserSettings|ApplySettings _returnvalue true))
    (:then_2
      (Utilities|FlowControl|Delay 3.0)
      (if (Variables|/Game/Characters/ThirdPerson/ThirdPersonBP/Blueprints/ThirdPersonCharacter.ThirdPersonCharacter_C|GetbIsTutorial? (.AsThird%20Person%20Character (Utilities|Casting|CastToThirdPersonCharacter (Game|GetPlayerCharacter 0))))
        (bind _returnvalue_2 (UserInterface|CreateWidget "/Game/HUD/Tutorialhelps/Help1_PlayerCharacter.Help1_PlayerCharacter_C"))
        (UserInterface|Viewport|AddtoViewport _returnvalue_2 0)
        (Game|SetGamePaused true)
        (Utilities|FlowControl|Delay 0.1)
        (Widget|RemovefromParent _returnvalue_2)
        (bind _returnvalue_3 (UserInterface|CreateWidget "/Game/HUD/Tutorialhelps/Help2_Enemy.Help2_Enemy_C"))
        (UserInterface|Viewport|AddtoViewport _returnvalue_3 0)
        (Game|SetGamePaused true)
        (Utilities|FlowControl|Delay 0.1)
        (Widget|RemovefromParent _returnvalue_3)
        (bind _returnvalue_4 (UserInterface|CreateWidget "/Game/HUD/Tutorialhelps/Help3_Goal.Help3_Goal_C"))
        (UserInterface|Viewport|AddtoViewport _returnvalue_4 0)
        (Game|SetGamePaused true)
        (Utilities|FlowControl|Delay 0.1)
        (Widget|RemovefromParent _returnvalue_4)))))

(event EventTick
  (params (DeltaSeconds :type Float%20%28single-precision%29)))

(fn ConstructionScript)